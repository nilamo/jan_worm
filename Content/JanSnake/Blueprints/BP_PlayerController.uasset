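; Player controller for a snake game that steers a worm by tilting the device and builds it from spawned BP_WormBodySegment actors.
; Each tick it averages the current and previous motion-sensor gravity vectors into a yaw heading.
; Separate timers add a head segment along that heading and remove the tail at half that rate, so the worm keeps growing.
; TriggerEndGame halts everything by disabling tick.
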(event `self.ReceiveBeginPlay`
  (bind _returnvalue (`|SpawnActorFromClass` "/Game/JanSnake/Blueprints/BP_WormBodySegment.BP_WormBodySegment_C" (`KismetMathLibrary.MakeTransform` (0.0 0.0 0.0)) "Undefined" "OverrideRootScale" null null))
  (`KismetArrayLibrary.Array_Add` (`self.Segments`) _returnvalue))

(event `self.ReceiveTick`
  (params (DeltaSeconds :type "Float (single-precision)"))
  (bind (_gravitydirection_roll _gravitydirection_pitch _gravitydirection_yaw) (`KismetMathLibrary.BreakRotator` (`self.GravityDirection`)))
  (bind _segments (`self.Segments`))
  (bind _segments_2 (`self.Segments`))
  (`|ExecutionSequence`
    (:`then_0`
      (`self.UpdateRotation`))
    (:`then_1`
      (bind _isreadytomove (`self.IsReadyToMove` DeltaSeconds))
      (if _isreadytomove
        (bind _returnvalue (`|SpawnActorFromClass` "/Game/JanSnake/Blueprints/BP_WormBodySegment.BP_WormBodySegment_C" (`KismetMathLibrary.MakeTransform` (+ (`self.K2_GetActorLocation` (`|GetArrayItem` _segments (`KismetArrayLibrary.Array_LastIndex` _segments))) (* (`KismetMathLibrary.GetForwardVector` (`KismetMathLibrary.MakeRotator` 0.0 0.0 _gravitydirection_yaw)) 50.0)) (`KismetMathLibrary.MakeRotator` 0.0 0.0 _gravitydirection_yaw)) "Undefined" "OverrideRootScale" null null))
        (`KismetArrayLibrary.Array_Add` (`self.Segments`) _returnvalue)))
    (:`then_2`
      (bind _is_ready_to_shorten (`self.IsReadyToShortain` DeltaSeconds))
      (if _is_ready_to_shorten
        (`self.K2_DestroyActor` (`|GetArrayItem` _segments_2))
        (`KismetArrayLibrary.Array_Remove` _segments_2)))))

(fn `IsReadyToMove`
  (params (`Delta Time` :type "Float (double-precision)"))
  (returns (IsReadyToMove :type Boolean))
  (bind _output_get (set `self.since_last_action` (+ `Delta Time` (`self.since_last_action`))))
  (if (>= _output_get (`self.action_threshold`))
    (set `self.since_last_action` 0.0)
    (return true)
    (else
      (return false))))

(fn `IsReadyToShortain`
  (params (`Delta Time` :type "Float (double-precision)"))
  (returns (`Is Ready To Shorten` :type Boolean))
  (bind _output_get (set `self.since_last_shorten` (+ `Delta Time` (`self.since_last_shorten`))))
  (if (> _output_get (`self.shorten_threshold`))
    (set `self.since_last_shorten` 0.0)
    (return true)
    (else
      (return false))))

(fn `TriggerEndGame`
  (`self.SetActorTickEnabled` false))

(fn `UpdateRotation`
  (bind (_tilt _rotationrate _gravity) (`self.GetInputMotionState`))
  (bind _returnvalue (`KismetMathLibrary.MakeVector` (* (.x _gravity) -1.0) (.y _gravity) (.z _gravity)))
  (bind (_returnvalue_roll _returnvalue_pitch _returnvalue_yaw) (`KismetMathLibrary.BreakRotator` (`KismetMathLibrary.MakeRotFromX` (`KismetMathLibrary.VLerp` _returnvalue (`self.last_gravity`) 0.5))))
  (`|ExecutionSequence`
    (:`then_0`
      (set `self.GravityDirection` (`KismetMathLibrary.MakeRotator` 0.0 0.0 _returnvalue_yaw)))
    (:`then_1`
      (set `self.last_gravity` _returnvalue))))

(fn `UserConstructionScript`
  (set `self.shorten_threshold` (* (`self.action_threshold`) 2.0)))